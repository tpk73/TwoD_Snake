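; Main controller for a grid-based Paper2D Snake game, spawning the HUD, snake head, food and border walls on play.
; Tick uses a Delay as the step timer, testing self, wall and food hits by location before applying gated directional input and moving segments tail-first.
; Eating adds score, a segment and new food while shortening the delay to a minimum.
; Death blanks the snake, shows game over and lets R reload the level.
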(event `Spawn New Snake Part`
  (params (SpawnLoc :type "Vector Structure") (isHead :type Boolean))
  ;[1 1 1] Spawn New Snake
  (bind _returnvalue (`|SpawnActorFromClass` "/Game/Assets/BP/BP_SnakeBody.BP_SnakeBody_C" (`KismetMathLibrary.MakeTransform` SpawnLoc) "AlwaysSpawn" "OverrideRootScale" null null))
  (`PaperFlipbookComponent.SetFlipbook` (`/Game/Assets/BP/BP_SnakeBody.PaperFlipbook` _returnvalue) (select `bool` isHead :`false` "/Game/Assets/Flipbooks/YellowSquare_Flipbook.YellowSquare_Flipbook" :`true` "/Game/Assets/Flipbooks/RedSquare_Flipbook.RedSquare_Flipbook" :!type "PaperFlipbook Object Reference"))
  (`KismetArrayLibrary.Array_Add` (`self.snakePartArray`) _returnvalue)
  (set `/Game/Assets/BP/BP_SnakeBody.isHead` isHead _returnvalue)
  (`self.K2_SetActorRotation` _returnvalue (`KismetMathLibrary.MakeRotator` 0.0 (select `int` (`KismetMathLibrary.RandomInteger` 3) :`0` 0.0 :`1` 90.0 :`2` 180.0 :`3` 270.0 :!type "Float (single-precision)")) false))

(event `Spawn Food`
  (bind _returnvalue (- (`self.zMax`) 100.0))
  (bind _returnvalue_2 (- (`self.xMax`) 100.0))
  ;[1 1 1] Spawn Food
  (bind _returnvalue_3 (`|SpawnActorFromClass` "/Game/Assets/BP/BP_Food.BP_Food_C" (`KismetMathLibrary.MakeTransform` (`KismetMathLibrary.MakeVector` (* (`.ReturnValue` (`KismetMathLibrary.FMod` (`KismetMathLibrary.RandomFloatInRange` (* _returnvalue_2 -1.0) _returnvalue_2) 100.0)) 100.0) -0.1 (* (`.ReturnValue` (`KismetMathLibrary.FMod` (`KismetMathLibrary.RandomFloatInRange` (* _returnvalue -1.0) _returnvalue) 100.0)) 100.0))) "AlwaysSpawn" "OverrideRootScale" null null))
  (set `self.foodActorRef` _returnvalue_3))

(event `Kill Snake`
  ;[1 1 1] Kill snake
  (set `self.isDead` true)
  (for (_array_element _array_index) (`self.snakePartArray`)
    (`PaperFlipbookComponent.SetFlipbook` (`/Game/Assets/BP/BP_SnakeBody.PaperFlipbook` _array_element) (select `bool` (== _array_index 0) :`false` "/Game/Assets/Flipbooks/Beath_Flipbook.Beath_Flipbook" :`true` "/Game/Assets/Flipbooks/Blank_Flipbook.Blank_Flipbook" :!type "PaperFlipbook Object Reference")))
  (`KismetSystemLibrary.Delay` 0.5)
  (for _array_element_2 (`self.snakePartArray`)
    (`PaperFlipbookComponent.SetFlipbook` (`/Game/Assets/BP/BP_SnakeBody.PaperFlipbook` _array_element_2) "/Game/Assets/Flipbooks/Blank_Flipbook.Blank_Flipbook")))

(event `Update Score`
  (params (Value :type Integer))
  ;[1 1 1] Update Score
  (bind _output_get (set `self.score` (+ Value (`self.score`))))
  (`/Game/Assets/BP/BP_UI_HUD.Update Score` (`self.HUDref`) _output_get))

(event `self.ReceiveBeginPlay`
  (bind (_remainder _returnvalue) (`KismetMathLibrary.FMod` (`self.zMax`) 50.0))
  (bind (_remainder_2 _returnvalue_2) (`KismetMathLibrary.FMod` (`self.xMax`) 50.0))
  ;[1 1 1] Init Game
  (bind _returnvalue_3 (`|CreateWidget` "/Game/Assets/BP/BP_UI_HUD.BP_UI_HUD_C"))
  (bind _output_get (set `self.HUDref` _returnvalue_3))
  (`UserWidget.AddToViewport` _output_get 0)
  (switch `int` (`KismetMathLibrary.RandomInteger` 3)
    (:`0`
      (set `self.Dir X` 1))
    (:`1`
      (set `self.Dir X` -1))
    (:`2`
      (set `self.Dir Z` 1))
    (:`3`
      (set `self.Dir Z` -1)))
  (set `self.delay` 0.2)
  (`KismetArrayLibrary.Array_Clear` (`self.snakePartArray`))
  (`self.Spawn New Snake Part` (0.0 0.0 0.0) true)
  (`self.Spawn Food`)
  (for _index (range (* _returnvalue_2 _returnvalue))
    (bind _returnvalue_4 (/ _index _returnvalue))
    (bind _returnvalue_5 (mod _index _returnvalue))
    (if (or (== _returnvalue_4 0) (== _returnvalue_4 (- _returnvalue_2 1)) (== _returnvalue_5 0) (== _returnvalue_5 (- _returnvalue 1)))
      (bind _returnvalue_6 (`|SpawnActorFromClass` "/Game/Assets/BP/BP_Block.BP_Block_C" (`KismetMathLibrary.MakeTransform` (`KismetMathLibrary.MakeVector` (+ (* (`self.xMax`) -1.0) (* _returnvalue_4 100.0)) 0.0 (+ (* (`self.zMax`) -1.0) (* _returnvalue_5 100.0)))) "AdjustIfPossibleButDontSpawnIfColliding" "OverrideRootScale" null null))
      (`KismetArrayLibrary.Array_Add` (`self.wallBlockArr`) _returnvalue_6))))

(event `Key|R`
  (params (Key :type "Key Structure"))
  (:`Pressed`
    (goto _label :!via `Open`)))

(event `Break self collision test loop`
  (goto _label_2 :!via `Break`))

(event `Break Wall Collision Test Loop`
  (goto _label_3 :!via `Break`))

(event `self.ReceiveTick`
  (params (DeltaSeconds :type "Float (single-precision)"))
  (bind _snakepartarray (`self.snakePartArray`))
  (if (`self.isDead`)
    (`/Engine/EditorBlueprintResources/StandardMacros.Gate` true :!label _label
      (:`Exit`
        (`/Engine/EditorBlueprintResources/StandardMacros.DoOnce` false
          (:`Completed`
            (`Widget.RemoveFromParent` (`self.HUDref`))
            (bind _returnvalue (`GameplayStatics.GetCurrentLevelName` true))
            (`GameplayStatics.OpenLevel` (`KismetStringLibrary.Conv_StringToName` _returnvalue))))))
    (else
      (`KismetSystemLibrary.Delay` (`self.delay`))
      (`|ExecutionSequence`
        (:`then_0`
          (for (_array_element _array_index) (`self.snakePartArray`) :!label _label_2
            (if (!= _array_index 0)
              (if (== (`self.K2_GetActorLocation` _array_element) (`self.K2_GetActorLocation` (`|GetArrayItem` (`self.snakePartArray`))))
                (`self.Kill Snake`)
                (`/Game/Assets/BP/BP_UI_HUD.GameOver` (`self.HUDref`))
                (`self.Break self collision test loop`))))
          (for _array_element_2 (`self.wallBlockArr`) :!label _label_3
            (if (== (`self.K2_GetActorLocation` _array_element_2) (`self.K2_GetActorLocation` (`|GetArrayItem` (`self.snakePartArray`))))
              (`self.Kill Snake`)
              (`/Game/Assets/BP/BP_UI_HUD.GameOver` (`self.HUDref`))
              (`self.Break Wall Collision Test Loop`))))
        (:`then_1`
          (if (not (`self.isDead`))
            (`|ExecutionSequence`
              (:`then_0`
                (if (== (`self.K2_GetActorLocation` (`|GetArrayItem` (`self.snakePartArray`))) (`self.K2_GetActorLocation` (`self.foodActorRef`)) :`ErrorTolerance` 1.0)
                  (`self.Update Score` (`/Game/Assets/BP/BP_Food.scoreVar` (`self.foodActorRef`)))
                  (`self.K2_DestroyActor` (`self.foodActorRef`))
                  (`self.Spawn New Snake Part` (`self.K2_GetActorLocation` (`|GetArrayItem` _snakepartarray (`KismetArrayLibrary.Array_LastIndex` _snakepartarray))))
                  (`self.Spawn Food`)
                  (set `self.delay` (`KismetMathLibrary.FClamp` (+ (`self.delay`) -0.01) 0.075 0.2))))
              (:`then_1`
                (`|ExecutionSequence`
                  (:`then_0`
                    (`/Engine/EditorBlueprintResources/StandardMacros.Gate` true :!label _label_4
                      (:`Exit`
                        (if (and (== (`self.Dir Z`) 0) (`self.canChangeDir`))
                          (set `self.Dir X` 0)
                          (set `self.Dir Z` 1)
                          (set `self.canChangeDir` false :!label _label_5)))))
                  (:`then_1`
                    (`/Engine/EditorBlueprintResources/StandardMacros.Gate` true :!label _label_6
                      (:`Exit`
                        (if (and (== (`self.Dir Z`) 0) (`self.canChangeDir`))
                          (set `self.Dir X` 0)
                          (set `self.Dir Z` -1)
                          (goto _label_5)))))
                  (:`then_2`
                    (`/Engine/EditorBlueprintResources/StandardMacros.Gate` true :!label _label_7
                      (:`Exit`
                        (if (and (== (`self.Dir X`) 0) (`self.canChangeDir`))
                          (set `self.Dir X` 1)
                          (set `self.Dir Z` 0)
                          (goto _label_5)))))
                  (:`then_3`
                    (`/Engine/EditorBlueprintResources/StandardMacros.Gate` true :!label _label_8
                      (:`Exit`
                        (if (and (== (`self.Dir X`) 0) (`self.canChangeDir`))
                          (set `self.Dir X` -1)
                          (set `self.Dir Z` 0)
                          (goto _label_5)))))
                  (:`then_4`
                    (for _index (range (`KismetArrayLibrary.Array_Length` (`self.snakePartArray`)))
                      (bind _returnvalue_2 (- (- (`KismetArrayLibrary.Array_Length` (`self.snakePartArray`)) 1) _index))
                      (if (`/Game/Assets/BP/BP_SnakeBody.isHead` (`|GetArrayItem` (`self.snakePartArray`) _returnvalue_2))
                        (bind _output (`|GetArrayItem` (`self.snakePartArray`) _returnvalue_2))
                        (`self.K2_AddActorWorldOffset` _output (`KismetMathLibrary.MakeVector` (* (`self.Dir X`) 100.0) 0.0 (* (`self.Dir Z`) 100.0)) false false)
                        (else
                          (`self.K2_SetActorLocation` _output (`self.K2_GetActorLocation` (`|GetArrayItem` (`self.snakePartArray`) (- _returnvalue_2 1))) false false))))
                    (set `self.canChangeDir` true)))))))))))

(event `InputAction|Snake Up`
  (params (Key :type "Key Structure"))
  (:`Pressed`
    (goto _label_4 :!via `Open`))
  (:`Released`
    (goto _label_4 :!via `Close`)))

(event `InputAction|Snake Down`
  (params (Key :type "Key Structure"))
  (:`Pressed`
    (goto _label_6 :!via `Open`))
  (:`Released`
    (goto _label_6 :!via `Close`)))

(event `InputAction|Snake Right`
  (params (Key :type "Key Structure"))
  (:`Pressed`
    (goto _label_7 :!via `Open`))
  (:`Released`
    (goto _label_7 :!via `Close`)))

(event `InputAction|Snake Left`
  (params (Key :type "Key Structure"))
  (:`Pressed`
    (goto _label_8 :!via `Open`))
  (:`Released`
    (goto _label_8 :!via `Close`)))

(fn `UserConstructionScript`)