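; BP_Food is a food pickup whose score value drops the longer it exists.
; On BeginPlay, SetFood starts at Blue and steps through Purple and Red to Yellow, re-calling itself after progressively shorter delays.
; Each stage swaps FoodSprite to a different credit sprite and lowers ScoreVar, with Yellow as the final, lowest-value state.
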(event `self.ReceiveBeginPlay`
  (`self.Set Food` "NewEnumerator0"))

(event `Set Food`
  (params (Type :type "/Game/Assets/BP/FoodColor_Enum Enum" :default "NewEnumerator0"))
  (bind _foodsprite (`self.foodSprite`))
  (switch `/Game/Assets/BP/FoodColor_Enum` Type
    (:`NewEnumerator0`
      (`PaperSpriteComponent.SetSprite` _foodsprite "/Game/Assets/New_Textures/FirstOrderCredit.FirstOrderCredit")
      (set `self.scoreVar` 100)
      (`KismetSystemLibrary.Delay` 3.0)
      (`self.Set Food` "NewEnumerator1"))
    (:`NewEnumerator1`
      (`PaperSpriteComponent.SetSprite` _foodsprite "/Game/Assets/New_Textures/empirecredit.empirecredit")
      (set `self.scoreVar` 50)
      (`KismetSystemLibrary.Delay` 2.0)
      (`self.Set Food` "NewEnumerator2"))
    (:`NewEnumerator2`
      (`PaperSpriteComponent.SetSprite` _foodsprite "/Game/Assets/New_Textures/MandaloreCredit.MandaloreCredit")
      (set `self.scoreVar` 25)
      (`KismetSystemLibrary.Delay` 1.0)
      (`self.Set Food` "NewEnumerator3"))
    (:`NewEnumerator3`
      (`PaperSpriteComponent.SetSprite` _foodsprite "/Game/Assets/New_Textures/RebelCredit.RebelCredit")
      (set `self.scoreVar` 10))))

(fn `UserConstructionScript`)